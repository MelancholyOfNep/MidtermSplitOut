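; Main_GM, apparently the game mode for a brick-breaking game, owns the score and the in-game UI.
; On BeginPlay it creates a GameUI widget for the first player and adds it to the viewport.
; BrickBroken adds the current multiplier to the score and updates the widget, while each BallSpawned raises that multiplier by a fixed step.
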(event `self.ReceiveBeginPlay`
  (bind _returnvalue (`|CreateWidget` "/Game/Widgets/GameUI.GameUI_C" (`GameplayStatics.GetPlayerController` 0)))
  (`UserWidget.AddToViewport` _returnvalue 0))

(event `BrickBroken`
  (bind _output_get (set `self.Score` (+ (`self.Score`) (`self.ScoreMultiplier`))))
  (`/Game/Widgets/GameUI.UpdateScore` (stale `self.ReceiveBeginPlay` _returnvalue) _output_get))

(event `BallSpawned`
  (set `self.ScoreMultiplier` (+ (`self.ScoreMultiplier`) 5)))

(fn `UserConstructionScript`)