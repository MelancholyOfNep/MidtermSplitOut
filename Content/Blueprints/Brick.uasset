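; Breakable brick actor for a brick-breaker game that counts itself in Main_GM's Bricks total on BeginPlay.
; A hit on its static mesh reports BrickBroken to the game mode and destroys the brick, without checking what struck it.
; Four corner overlap components respond only to a BouncingBall, calling its CornerHit before reporting and destroying the brick the same way.
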(event `self.ReceiveBeginPlay`
  (bind _asmain_gm (cast `/Game/Blueprints/Old_shit_Im_to_scared_to_delete/Main_GM` (`GameplayStatics.GetGameMode`)))
  (set `/Game/Blueprints/Old_shit_Im_to_scared_to_delete/Main_GM.Bricks` (+ 1 (`/Game/Blueprints/Old_shit_Im_to_scared_to_delete/Main_GM.Bricks` _asmain_gm)) _asmain_gm))

(event `self.Corner1.OnComponentBeginOverlap`
  (params (OverlappedComponent :type "PrimitiveComponent Object Reference") (OtherActor :type "Actor Object Reference") (OtherComp :type "PrimitiveComponent Object Reference") (OtherBodyIndex :type Integer) (bFromSweep :type Boolean) (SweepResult :type "HitResult Structure (by ref)"))
  (bind _asbouncing_ball (cast `/Game/Blueprints/BouncingBall` OtherActor))
  (`/Game/Blueprints/BouncingBall.CornerHit` _asbouncing_ball)
  (bind _asmain_gm (cast `/Game/Blueprints/Old_shit_Im_to_scared_to_delete/Main_GM` (`GameplayStatics.GetGameMode`)))
  (`/Game/Blueprints/Old_shit_Im_to_scared_to_delete/Main_GM.BrickBroken` _asmain_gm)
  (`self.K2_DestroyActor`))

(event `self.StaticMeshComponent.OnComponentHit`
  (params (HitComponent :type "PrimitiveComponent Object Reference") (OtherActor :type "Actor Object Reference") (OtherComp :type "PrimitiveComponent Object Reference") (NormalImpulse :type "Vector Structure") (Hit :type "HitResult Structure (by ref)"))
  (bind _asmain_gm (cast `/Game/Blueprints/Old_shit_Im_to_scared_to_delete/Main_GM` (`GameplayStatics.GetGameMode`)))
  (`/Game/Blueprints/Old_shit_Im_to_scared_to_delete/Main_GM.BrickBroken` _asmain_gm)
  (`self.K2_DestroyActor`))

(event `self.Corner2.OnComponentBeginOverlap`
  (params (OverlappedComponent :type "PrimitiveComponent Object Reference") (OtherActor :type "Actor Object Reference") (OtherComp :type "PrimitiveComponent Object Reference") (OtherBodyIndex :type Integer) (bFromSweep :type Boolean) (SweepResult :type "HitResult Structure (by ref)"))
  (bind _asbouncing_ball (cast `/Game/Blueprints/BouncingBall` OtherActor))
  (`/Game/Blueprints/BouncingBall.CornerHit` _asbouncing_ball)
  (bind _asmain_gm (cast `/Game/Blueprints/Old_shit_Im_to_scared_to_delete/Main_GM` (`GameplayStatics.GetGameMode`)))
  (`/Game/Blueprints/Old_shit_Im_to_scared_to_delete/Main_GM.BrickBroken` _asmain_gm)
  (`self.K2_DestroyActor`))

(event `self.Corner3.OnComponentBeginOverlap`
  (params (OverlappedComponent :type "PrimitiveComponent Object Reference") (OtherActor :type "Actor Object Reference") (OtherComp :type "PrimitiveComponent Object Reference") (OtherBodyIndex :type Integer) (bFromSweep :type Boolean) (SweepResult :type "HitResult Structure (by ref)"))
  (bind _asbouncing_ball (cast `/Game/Blueprints/BouncingBall` OtherActor))
  (`/Game/Blueprints/BouncingBall.CornerHit` _asbouncing_ball)
  (bind _asmain_gm (cast `/Game/Blueprints/Old_shit_Im_to_scared_to_delete/Main_GM` (`GameplayStatics.GetGameMode`)))
  (`/Game/Blueprints/Old_shit_Im_to_scared_to_delete/Main_GM.BrickBroken` _asmain_gm)
  (`self.K2_DestroyActor`))

(event `self.Corner4.OnComponentBeginOverlap`
  (params (OverlappedComponent :type "PrimitiveComponent Object Reference") (OtherActor :type "Actor Object Reference") (OtherComp :type "PrimitiveComponent Object Reference") (OtherBodyIndex :type Integer) (bFromSweep :type Boolean) (SweepResult :type "HitResult Structure (by ref)"))
  (bind _asbouncing_ball (cast `/Game/Blueprints/BouncingBall` OtherActor))
  (`/Game/Blueprints/BouncingBall.CornerHit` _asbouncing_ball)
  (bind _asmain_gm (cast `/Game/Blueprints/Old_shit_Im_to_scared_to_delete/Main_GM` (`GameplayStatics.GetGameMode`)))
  (`/Game/Blueprints/Old_shit_Im_to_scared_to_delete/Main_GM.BrickBroken` _asmain_gm)
  (`self.K2_DestroyActor`))

(fn `UserConstructionScript`)