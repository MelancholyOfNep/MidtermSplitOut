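; Bouncing ball that moves on the X/Z plane and costs the player the game if it falls below the play area.
; Tick runs four bound checks, flipping the matching BallMovement velocity component at the side and top limits.
; Below the bottom limit, it applies a clear material, spawns an explosion and opens GameOver after a delay.
; A CornerHit event reverses both axes, and the construction script stores a dynamic material as BallColor.
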(event `self.ReceiveTick`
  (params (DeltaSeconds :type "Float (single-precision)"))
  ;[1 1 1] Check to see if the ball has hit any bounds, and bounce / fail if so
  (`|ExecutionSequence`
    (:`then_0`
      (`self.X+ Bound for ball`))
    (:`then_1`
      (`self.X- Bound for Ball`))
    (:`then_2`
      (`self.Z+ Bound for Ball`))
    (:`then_3`
      (`self.Z- Bound for Ball`))))

(event `X+ Bound for ball`
  (bind _ball_movement (`self.Ball Movement`))
  ;[1 1 1] Right-side bound for ball
  (`/Engine/EditorBlueprintResources/StandardMacros.CompareFloat` (.x (`SceneComponent.K2_GetComponentLocation` (`self.Ball`))) 600.0
    (:`>`
      (set `MovementComponent.Velocity` (`KismetMathLibrary.MakeVector` (* (.x (`MovementComponent.Velocity` _ball_movement)) -1.0) (.y (`MovementComponent.Velocity` _ball_movement)) (.z (`MovementComponent.Velocity` _ball_movement))) _ball_movement))))

(event `X- Bound for Ball`
  (bind _ball_movement (`self.Ball Movement`))
  ;[1 1 1] Left-side bound for ball
  (`/Engine/EditorBlueprintResources/StandardMacros.CompareFloat` (.x (`SceneComponent.K2_GetComponentLocation` (`self.Ball`))) -600.0
    (:`<`
      (set `MovementComponent.Velocity` (`KismetMathLibrary.MakeVector` (* (.x (`MovementComponent.Velocity` _ball_movement)) -1.0) (.y (`MovementComponent.Velocity` _ball_movement)) (.z (`MovementComponent.Velocity` _ball_movement))) _ball_movement))))

(event `Z+ Bound for Ball`
  (bind _ball_movement (`self.Ball Movement`))
  ;[1 1 1] Upper bound for ball
  (`/Engine/EditorBlueprintResources/StandardMacros.CompareFloat` (.z (`SceneComponent.K2_GetComponentLocation` (`self.Ball`))) 720.0
    (:`>`
      (set `MovementComponent.Velocity` (`KismetMathLibrary.MakeVector` (.x (`MovementComponent.Velocity` _ball_movement)) (.y (`MovementComponent.Velocity` _ball_movement)) (* (.z (`MovementComponent.Velocity` _ball_movement)) -1.0)) _ball_movement))))

(event `Z- Bound for Ball`
  (bind _ball (`self.Ball`))
  ;[1 1 1] When the player loses, spawn a particle effect explosion, wait a second (maybe fade to black?), and open the game over level
  (`/Engine/EditorBlueprintResources/StandardMacros.CompareFloat` (.z (`SceneComponent.K2_GetComponentLocation` _ball)) -50.0
    (:`<`
      (`PrimitiveComponent.SetMaterial` _ball 0 "/Game/Materials/Ball_Clear_Mat.Ball_Clear_Mat")
      (`GameplayStatics.SpawnEmitterAtLocation` "/Game/StarterContent/Particles/P_Explosion.P_Explosion" (`SceneComponent.K2_GetComponentLocation` _ball) :!pinned true) ; Maybe replace me with a non-included effect.
      (`KismetSystemLibrary.Delay` 1.0)
      (`GameplayStatics.OpenLevel` "GameOver"))))

(event `CornerHit`
  (bind _ball_movement (`self.Ball Movement`))
  (set `MovementComponent.Velocity` (`KismetMathLibrary.MakeVector` (* (.x (`MovementComponent.Velocity` _ball_movement)) -1.0) (.y (`MovementComponent.Velocity` _ball_movement)) (* (.z (`MovementComponent.Velocity` _ball_movement)) -1.0)) _ball_movement))

(fn `UserConstructionScript`
  (bind _returnvalue (`PrimitiveComponent.CreateDynamicMaterialInstance` (`self.Ball`) 0 null "None"))
  (set `self.Ball Color` _returnvalue))