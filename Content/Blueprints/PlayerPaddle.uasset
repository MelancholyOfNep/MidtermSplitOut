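; Player-controlled paddle that slides along the world X axis, spawns balls and handles pausing.
; Left and right input axes feed movement input, while Tick runs two checks that snap the paddle back within symmetric X bounds.
; The SpawnBall action spawns an actor just above the Cube component, unless it would collide.
; The P key toggles game pause, the mouse cursor and a Pause widget created on demand.
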(event `InputAxis|Move Right`
  (params (AxisValue :type "Float (single-precision)"))
  ;[1 1 1] Player Movement
  (`self.AddMovementInput` (1.0 0.0 0.0) AxisValue))

(event `InputAxis|Move Left`
  (params (AxisValue :type "Float (single-precision)"))
  ;[1 1 1] Player Movement
  (`self.AddMovementInput` (1.0 0.0 0.0) AxisValue))

(event `self.ReceiveTick`
  (params (DeltaSeconds :type "Float (single-precision)"))
  ;[1 1 1] Bounds Hub
  (`|ExecutionSequence`
    (:`then_0`
      (`self.Get Positive X Bounds`))
    (:`then_1`
      (`self.Get Negative X Bounds`))))

(event `Get Positive X Bounds`
  ;[1 1 1] Bounds
  ;;[1 1 1] Positive X Axis
  (`/Engine/EditorBlueprintResources/StandardMacros.CompareFloat` (.x (`SceneComponent.K2_GetComponentLocation` (`self.Player Character`))) 550.0
    (:`>`
      (`self.K2_SetActorLocation` (`KismetMathLibrary.MakeVector` 550.0 (.y (`SceneComponent.K2_GetComponentLocation` (`self.Player Character`))) (.z (`SceneComponent.K2_GetComponentLocation` (`self.Player Character`))))))))

(event `Get Negative X Bounds`
  ;[1 1 1] Bounds
  ;;[1 1 1] Negative X Axis
  (`/Engine/EditorBlueprintResources/StandardMacros.CompareFloat` (.x (`SceneComponent.K2_GetComponentLocation` (`self.Player Character`))) -550.0
    (:`<`
      (`self.K2_SetActorLocation` (`KismetMathLibrary.MakeVector` -550.0 (.y (`SceneComponent.K2_GetComponentLocation` (`self.Player Character`))) (.z (`SceneComponent.K2_GetComponentLocation` (`self.Player Character`))))))))

(event `Key|P` :paused true
  (params (Key :type "Key Structure"))
  (bind _returnvalue (`GameplayStatics.GetPlayerController` 0))
  ;[1 1 1] Pauses the game.
  (:`Pressed`
    (if (`self.IsPaused`)
      (set `self.IsPaused` false)
      (`GameplayStatics.SetGamePaused` false)
      (set `PlayerController.bShowMouseCursor` false _returnvalue)
      ;[1 1 1] Creates pause screen
      (`Widget.RemoveFromParent` (stale _returnvalue_2))
      (else
        (set `self.IsPaused` true)
        (`GameplayStatics.SetGamePaused` true)
        (set `PlayerController.bShowMouseCursor` true _returnvalue)
        (bind _returnvalue_2 (`|CreateWidget` "/Game/Widgets/Pause.Pause_C"))
        (`UserWidget.AddToViewport` _returnvalue_2 0)))))

(event `InputAction|SpawnBall`
  (params (Key :type "Key Structure"))
  ;[1 1 1] Spawn ball
  (:`Pressed`
    (`|SpawnActorFromClass` "/Game/Blueprints/BouncingBall.BouncingBall_C" (`KismetMathLibrary.Conv_VectorToTransform` (+ (`SceneComponent.K2_GetComponentLocation` (`self.Cube`)) (0.0 0.0 30.0))) "DontSpawnIfColliding" "OverrideRootScale" null null)))

(fn `UserConstructionScript`)